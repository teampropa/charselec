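; BP_NoteBlock is a rhythm-game note actor that travels along one of four tracks and can be hit by the player.
; Construction picks a themed mesh (broom, pot, laptop, dumbbell) from TrackNumber.
; Tick offsets the mesh along negative local X, scaled by distance to NoteTargetActor over Delay.
; Hit-note destroys it once an overlap has begun, while ending an overlap increments the GameInstance mistake count and destroys it.
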(event `self.ReceiveTick`
  (params (DeltaSeconds :type "Float (single-precision)"))
  ; Move noteblock
  (`SceneComponent.K2_AddLocalOffset` (`self.Cube`) (`KismetMathLibrary.MakeVector` (* (* (/ (`self.GetDistanceTo` (`self.NoteTargetActor`)) (`self.Delay`)) (`GameplayStatics.GetWorldDeltaSeconds`)) -1.0)) false false))

(event `self.ReceiveActorEndOverlap`
  (params (OtherActor :type "Actor Object Reference"))
  ; Destroy noteblock
  (bind _asdata__game_instance (cast `/Game/char-select/Data-Game-instance` (`GameplayStatics.GetGameInstance`)))
  (set `/Game/char-select/Data-Game-instance.game-mistakes` (+ (`/Game/char-select/Data-Game-instance.game-mistakes` _asdata__game_instance) 1) _asdata__game_instance)
  (`KismetSystemLibrary.Delay` 0.0)
  (`self.K2_DestroyActor`))

(event `self.ReceiveActorBeginOverlap`
  (params (OtherActor :type "Actor Object Reference"))
  (set `self.overlap` true))

(event `/Game/char-select/Interface-char-select.hit-note`
  (if (`self.overlap`)
    (`self.K2_DestroyActor`)))

(fn `get-char`
  (returns (`char-output` :type "Array of /Game/char-select/char-select Object Reference"))
  (return))

(fn `SetTrack1Assets`
  (`StaticMeshComponent.SetStaticMesh` (`self.Cube`) "/Game/Layout-assets/Notes/broom_notes/Buttons_for_Notes（Broom__update2.Buttons_for_Notes（Broom__update2"))

(fn `SetTrack2Assets`
  (`StaticMeshComponent.SetStaticMesh` (`self.Cube`) "/Game/Layout-assets/Notes/Egg_notes/Buttons_for_Notes（Pot__update2.Buttons_for_Notes（Pot__update2"))

(fn `SetTrack3Assets`
  (`StaticMeshComponent.SetStaticMesh` (`self.Cube`) "/Game/Layout-assets/Notes/laptop_notes/Buttons_for_Notes（Laptop__update.Buttons_for_Notes（Laptop__update"))

(fn `SetTrack4Assets`
  (`StaticMeshComponent.SetStaticMesh` (`self.Cube`) "/Game/Layout-assets/Notes/dumbell_notes/Buttons_for_Notes（Dumball__update.Buttons_for_Notes（Dumball__update"))

(fn `UserConstructionScript`
  (switch `int` (`self.TrackNumber`)
    (:`0`
      (`self.SetTrack1Assets`))
    (:`1`
      (`self.SetTrack2Assets`))
    (:`2`
      (`self.SetTrack3Assets`))
    (:`3`
      (`self.SetTrack4Assets`))))