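; BP_NoteCollider is an actor, apparently for a rhythm game, that tracks note overlaps on its Collider to score hits.
; Begin overlap clears IsNoteHitting and records StartTime, while end overlap sets the flag.
; While the flag is set, Tick stores Distance as the actor's own Y location minus itself, so zero as written.
; GetPointsForNote returns truncated Distance when flagged, otherwise -1; Getchar is an empty stub.
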(event `self.ReceiveTick`
  (params (DeltaSeconds :type "Float (single-precision)"))
  (if (`self.IsNoteHitting`)
    (set `self.Distance` (- (.y (.location (`self.GetTransform`))) (.y (.location (`self.GetTransform`)))))))

(event `self.Collider.OnComponentEndOverlap`
  (params (OverlappedComponent :type "PrimitiveComponent Object Reference") (OtherActor :type "Actor Object Reference") (OtherComp :type "PrimitiveComponent Object Reference") (OtherBodyIndex :type Integer))
  (set `self.IsNoteHitting` true))

(event `self.Collider.OnComponentBeginOverlap`
  (params (OverlappedComponent :type "PrimitiveComponent Object Reference") (OtherActor :type "Actor Object Reference") (OtherComp :type "PrimitiveComponent Object Reference") (OtherBodyIndex :type Integer) (bFromSweep :type Boolean) (SweepResult :type "HitResult Structure (by ref)"))
  (set `self.IsNoteHitting` false)
  (set `self.StartTime` (`KismetSystemLibrary.GetGameTimeInSeconds`)))

(fn `get-char`
  (returns (`char-output` :type "Array of /Game/char-select/char-select Object Reference"))
  (return))

(fn `GetPointsForNote`
  (returns (Points :type Integer))
  (if (`self.IsNoteHitting`)
    (return (`KismetMathLibrary.FTrunc` (`self.Distance`)))
    (else
      (return -1))))

(fn `UserConstructionScript`)