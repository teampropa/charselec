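; BP_NoteCollider_2 is a rhythm-game hit zone that rates note timing for the second collider slot.
; While a note overlaps, Tick writes its signed distance to Data-Game-instance, deriving the sign from distances to world origin.
; Hit-note destroys the note, and GetPointsForNote converts distance into points.
; Overlap end spawns jittered Early, Goodjob, Late or Miss feedback, counts misses as mistakes, and clears Notecollide1 rather than Notecollide2.
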(event `self.ReceiveTick`
  (params (DeltaSeconds :type "Float (single-precision)"))
  (bind _returnvalue_location (`KismetMathLibrary.BreakTransform` (`self.GetTransform`)))
  ; hit calculator
  (if (`self.IsNoteHitting`)
    (bind _returnvalue (`SceneComponent.K2_GetComponentLocation` (stale `self.Collider.OnComponentBeginOverlap` OtherComp)))
    (if (> (`KismetMathLibrary.VSize` _returnvalue) (`KismetMathLibrary.VSize` _returnvalue_location))
      (bind _returnvalue_2 (`KismetMathLibrary.VSize` (- _returnvalue _returnvalue_location)))
      (set `self.Distance` _returnvalue_2)
      (else
        (set `self.Distance` (* _returnvalue_2 -1.0))))
    (bind _asdata__game_instance (cast `/Game/char-select/Data-Game-instance` (`GameplayStatics.GetGameInstance`)))
    (set `/Game/char-select/Data-Game-instance.note-collide-2` true _asdata__game_instance)
    (set `/Game/char-select/Data-Game-instance.Distance-global-2` (`self.Distance`) _asdata__game_instance)
    (else
      (bind _asdata__game_instance_2 (cast `/Game/char-select/Data-Game-instance` (`GameplayStatics.GetGameInstance`)))
      (set `/Game/char-select/Data-Game-instance.Distance-global-2` 100.0 _asdata__game_instance_2))))

(event `self.Collider.OnComponentBeginOverlap`
  (params (OverlappedComponent :type "PrimitiveComponent Object Reference") (OtherActor :type "Actor Object Reference") (OtherComp :type "PrimitiveComponent Object Reference") (OtherBodyIndex :type Integer) (bFromSweep :type Boolean) (SweepResult :type "HitResult Structure (by ref)"))
  ; hit calculator
  (set `self.IsNoteHitting` true)
  (set `self.StartTime` (`KismetSystemLibrary.GetGameTimeInSeconds`)))

(event `/Game/char-select/Interface-char-select.hit-note`
  (`/Engine/EditorBlueprintResources/StandardMacros.IsValid` (stale `self.Collider.OnComponentBeginOverlap` OtherActor)
    (:`Is Valid`
      (`self.K2_DestroyActor` (stale `self.Collider.OnComponentBeginOverlap` OtherActor)))))

(event `self.Collider.OnComponentEndOverlap`
  (params (OverlappedComponent :type "PrimitiveComponent Object Reference") (OtherActor :type "Actor Object Reference") (OtherComp :type "PrimitiveComponent Object Reference") (OtherBodyIndex :type Integer))
  (bind (_returnvalue_x _returnvalue_y _returnvalue_z) (`KismetMathLibrary.BreakVector` (`SceneComponent.K2_GetComponentLocation` OtherComp)))
  (bind (_returnvalue_x_2 _returnvalue_y_2 _returnvalue_z_2) (`KismetMathLibrary.BreakVector` (`SceneComponent.K2_GetComponentLocation` OtherComp)))
  (bind (_returnvalue_x_3 _returnvalue_y_3 _returnvalue_z_3) (`KismetMathLibrary.BreakVector` (`SceneComponent.K2_GetComponentLocation` OtherComp)))
  (bind (_returnvalue_x_4 _returnvalue_y_4 _returnvalue_z_4) (`KismetMathLibrary.BreakVector` (`SceneComponent.K2_GetComponentLocation` OtherComp)))
  ; Spawn Feedback
  (set `self.IsNoteHitting` false)
  (bind _asdata__game_instance (cast `/Game/char-select/Data-Game-instance` (`GameplayStatics.GetGameInstance`)))
  (set `/Game/char-select/Data-Game-instance.note-collide-1` false _asdata__game_instance)
  (if (`KismetMathLibrary.InRange_FloatFloat` (`self.Distance`) 11.0 26.5)
    (`|SpawnActorFromClass` "/Game/Layout-assets/Fonts/early.early_C" (`KismetMathLibrary.MakeTransform` (`KismetMathLibrary.MakeVector` (+ _returnvalue_x -30.0) (+ _returnvalue_y (`KismetMathLibrary.RandomFloatInRange` -20.0 20.0)) (+ _returnvalue_z (`KismetMathLibrary.RandomFloatInRange` -20.0 20.0)))) "Undefined" "MultiplyWithRoot" null null)
    (elif (`KismetMathLibrary.InRange_FloatFloat` (`self.Distance`) -10.0 10.0)
      (`|SpawnActorFromClass` "/Game/Layout-assets/Fonts/good-job.good-job_C" (`KismetMathLibrary.MakeTransform` (`KismetMathLibrary.MakeVector` (+ _returnvalue_x_2 -30.0) (+ _returnvalue_y_2 (`KismetMathLibrary.RandomFloatInRange` -20.0 20.0)) (+ _returnvalue_z_2 (`KismetMathLibrary.RandomFloatInRange` -20.0 20.0)))) "Undefined" "MultiplyWithRoot" null null)
      (elif (`KismetMathLibrary.InRange_FloatFloat` (`self.Distance`) -26.5 -11.0)
        (`|SpawnActorFromClass` "/Game/Layout-assets/Fonts/late.late_C" (`KismetMathLibrary.MakeTransform` (`KismetMathLibrary.MakeVector` (+ _returnvalue_x_3 -30.0) (+ _returnvalue_y_3 (`KismetMathLibrary.RandomFloatInRange` -20.0 20.0)) (+ _returnvalue_z_3 (`KismetMathLibrary.RandomFloatInRange` -20.0 20.0)))) "Undefined" "MultiplyWithRoot" null null)
        (else
          (`|SpawnActorFromClass` "/Game/Layout-assets/Fonts/miss.miss_C" (`KismetMathLibrary.MakeTransform` (`KismetMathLibrary.MakeVector` (+ _returnvalue_x_4 -30.0) (+ _returnvalue_y_4 (`KismetMathLibrary.RandomFloatInRange` -20.0 20.0)) (+ _returnvalue_z_4 (`KismetMathLibrary.RandomFloatInRange` -20.0 20.0)))) "Undefined" "MultiplyWithRoot" null null)
          (bind _asdata__game_instance_2 (cast `/Game/char-select/Data-Game-instance` (`GameplayStatics.GetGameInstance`)))
          (set `/Game/char-select/Data-Game-instance.game-mistakes` (+ (`/Game/char-select/Data-Game-instance.game-mistakes` _asdata__game_instance_2) 1) _asdata__game_instance_2))))))

(fn `get-char`
  (returns (`char-output` :type "Array of /Game/char-select/char-select Object Reference"))
  (return))

(fn `GetPointsForNote`
  (returns (Points :type Integer))
  (if (`self.IsNoteHitting`)
    (return (`KismetMathLibrary.FTrunc` (`KismetMathLibrary.FMax` (+ (* (`self.Distance`) -1.0) 10.0))))
    (else
      (return -1))))

(fn `UserConstructionScript`)