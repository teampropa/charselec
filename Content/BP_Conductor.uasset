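; BP_Conductor is a rhythm-game conductor that starts music on input and spawns colored note blocks in four columns from MIDI.
; MIDI events are filtered by channel and note, with counters passing every fifth event; MetaSound watcher bindings exist but are unwired.
; Five seconds after playback or a clock event, it spawns A_Articles, clears blocks and pauses.
; A looping timeline prunes invalid blocks, and Game-lose destroys all blocks and itself.
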(event `MidiClockEvent`
  (params (OutputName :type Name) (Output :type "MetaSoundOutput Structure (by ref)"))
  ; Pause Function
  (bind (_success _returnvalue) (`MusicTimestampBlueprintLibrary.GetMusicTimestamp` Output))
  (`KismetSystemLibrary.Delay` 5.0 :!label _label)
  (if true
    (`/Engine/EditorBlueprintResources/StandardMacros.DoOnce` false :!label _label_2
      (:`Completed`
        (`|SpawnActorFromClass` "/Game/Article/A_Articles.A_Articles_C" (`KismetMathLibrary.Conv_VectorToTransform` (`self.K2_GetActorLocation`)) "Undefined" "MultiplyWithRoot" null null)
        (`self.DestroyNoteBlocks`)
        (`GameplayStatics.SetGamePaused` true)
        (goto _label_2 :!via `Reset`)))))

(event `self.ReceiveBeginPlay`
  (bind _returnvalue (`GameplayStatics.GetPlayerController` 0))
  (bind _noteblocks (`self.NoteBlocks`))
  ; setup
  (bind _asplayer__controller (cast `/Game/Game-mode/Player-Controller` _returnvalue))
  (`EnhancedInputSubsystemInterface.AddMappingContext` (pcsubsystem `EnhancedInputLocalPlayerSubsystem` _asplayer__controller) "/Game/Game-mode/Inputs.Inputs" 0 (struct))
  (`self.EnableInput` _returnvalue)
  (`AudioComponent.Stop` (`self.Audio`))
  (`Timeline|Timeline` :!label _label_3
    (:`Finished`
      (for _array_element _noteblocks
        (if (not (`KismetSystemLibrary.IsValid` _array_element))
          (`KismetArrayLibrary.Array_RemoveItem` _noteblocks _array_element)))
      (`KismetSystemLibrary.PrintString` (`KismetStringLibrary.Concat_StrStr` "Array Length after cleanup: " (`KismetStringLibrary.Conv_IntToString` (`KismetArrayLibrary.Array_Length` _noteblocks))))
      (goto _label_3 :!via `PlayFromStart`))))

(event `EnhancedInput|/Game/Game-mode/Input-Actions/input-column-3`
  (params (ActionValue :type Boolean) (ElapsedSeconds :type "Float (double-precision)") (TriggeredSeconds :type "Float (double-precision)") (InputAction :type "InputAction Object Reference" :default "/Game/Game-mode/Input-Actions/input-column-3.input-column-3"))
  ; start game
  (:`Started`
    (`self.DisableInput` null)
    (`KismetSystemLibrary.Delay` 1.0)
    (`AudioComponent.Play` (`self.Audio`) 0.0)
    (goto _label)))

(event `OnMidiReceived`
  (params (OutputName :type Name) (Output :type "MetaSoundOutput Structure (by ref)"))
  (bind (_returnvalue_x _returnvalue_y _returnvalue_z) (`KismetMathLibrary.BreakVector` (`self.K2_GetActorLocation`)))
  ; Spawn notes
  (bind (_success _returnvalue) (`MidiEventInfoBlueprintLibrary.GetMidiEventInfo` Output))
  (if _success
    (bind _returnvalue_2 (`MidiEventInfoBlueprintLibrary.GetChannel` _returnvalue))
    (if (`KismetArrayLibrary.Array_Contains` (`self.column 1 channel`) _returnvalue_2)
      (`|ExecutionSequence`
        (:`then_0`
          (set `self.note timer 1` (+ (`self.note timer 1`) 1))
          (if (> (`self.note timer 1`) 4)
            (set `self.note timer 1` 0)))
        (:`then_1`
          (set `self.CurrentSpawnY` (+ _returnvalue_y -105.0))
          (set `self.CurrentSpawnColor` (struct :`R` 1.0 :`A` 1.0))
          (`MidiEventInfoBlueprintLibrary.IsNoteOn` _returnvalue)
          (if (== (`self.note timer 1`) 4)
            (bind _returnvalue_3 (`MidiEventInfoBlueprintLibrary.GetNoteNumber` _returnvalue))
            (if (`KismetArrayLibrary.Array_Contains` (`self.column 1 note`) _returnvalue_3)
              (bind _returnvalue_4 (`|SpawnActorFromClass` "/Game/BP_NoteBlock_1.BP_NoteBlock_1_C" (`KismetMathLibrary.MakeTransform` (`KismetMathLibrary.MakeVector` _returnvalue_x (`self.CurrentSpawnY`) _returnvalue_z)) "Undefined" "MultiplyWithRoot" self (struct) null))
              (`KismetArrayLibrary.Array_Add` (`self.NoteBlocks`) _returnvalue_4)))))
      (elif (`KismetArrayLibrary.Array_Contains` (`self.column 2 channel`) _returnvalue_2)
        (`|ExecutionSequence`
          (:`then_0`
            (set `self.note timer 2` (+ (`self.note timer 2`) 1))
            (if (> (`self.note timer 2`) 4)
              (set `self.note timer 2` 0)))
          (:`then_1`
            (set `self.CurrentSpawnY` (+ _returnvalue_y -35.0))
            (set `self.CurrentSpawnColor` (struct :`B` 1.0 :`A` 1.0))
            (`MidiEventInfoBlueprintLibrary.IsNoteOn` _returnvalue)
            (if (== (`self.note timer 2`) 4)
              (bind _returnvalue_5 (`MidiEventInfoBlueprintLibrary.GetNoteNumber` _returnvalue))
              (if (`KismetArrayLibrary.Array_Contains` (`self.column 2 note`) _returnvalue_5)
                (bind _returnvalue_6 (`|SpawnActorFromClass` "/Game/BP_NoteBlock_2.BP_NoteBlock_2_C" (`KismetMathLibrary.MakeTransform` (`KismetMathLibrary.MakeVector` _returnvalue_x (`self.CurrentSpawnY`) _returnvalue_z)) "Undefined" "MultiplyWithRoot" self (struct) null))
                (`KismetArrayLibrary.Array_Add` (`self.NoteBlocks`) _returnvalue_6)))))
        (elif (`KismetArrayLibrary.Array_Contains` (`self.column 3 channel`) _returnvalue_2)
          (`|ExecutionSequence`
            (:`then_0`
              (set `self.note timer 3` (+ (`self.note timer 3`) 1))
              (if (> (`self.note timer 3`) 4)
                (set `self.note timer 3` 0)))
            (:`then_1`
              (set `self.CurrentSpawnY` (+ _returnvalue_y 35.0))
              (set `self.CurrentSpawnColor` (struct :`G` 1.0 :`A` 1.0))
              (`MidiEventInfoBlueprintLibrary.IsNoteOn` _returnvalue)
              (if (== (`self.note timer 3`) 4)
                (bind _returnvalue_7 (`MidiEventInfoBlueprintLibrary.GetNoteNumber` _returnvalue))
                (if (`KismetArrayLibrary.Array_Contains` (`self.column 3 note`) _returnvalue_7)
                  (bind _returnvalue_8 (`|SpawnActorFromClass` "/Game/BP_NoteBlock_3.BP_NoteBlock_3_C" (`KismetMathLibrary.MakeTransform` (`KismetMathLibrary.MakeVector` _returnvalue_x (`self.CurrentSpawnY`) _returnvalue_z)) "Undefined" "MultiplyWithRoot" self (struct) null))
                  (`KismetArrayLibrary.Array_Add` (`self.NoteBlocks`) _returnvalue_8)))))
          (elif (`KismetArrayLibrary.Array_Contains` (`self.column 4 channel`) _returnvalue_2)
            (`|ExecutionSequence`
              (:`then_0`
                (set `self.note timer 4` (+ (`self.note timer 4`) 1))
                (if (> (`self.note timer 4`) 4)
                  (set `self.note timer 4` 0)))
              (:`then_1`
                (set `self.CurrentSpawnY` (+ _returnvalue_y 105.0))
                (set `self.CurrentSpawnColor` (struct :`R` 1.0 :`G` 1.0 :`A` 1.0))
                (`MidiEventInfoBlueprintLibrary.IsNoteOn` _returnvalue)
                (if (== (`self.note timer 4`) 4)
                  (bind _returnvalue_9 (`MidiEventInfoBlueprintLibrary.GetNoteNumber` _returnvalue))
                  (if (`KismetArrayLibrary.Array_Contains` (`self.column 4 note`) _returnvalue_9)
                    (bind _returnvalue_10 (`|SpawnActorFromClass` "/Game/BP_NoteBlock_4.BP_NoteBlock_4_C" (`KismetMathLibrary.MakeTransform` (`KismetMathLibrary.MakeVector` _returnvalue_x (`self.CurrentSpawnY`) _returnvalue_z)) "Undefined" "MultiplyWithRoot" self (struct) null))
                    (`KismetArrayLibrary.Array_Add` (`self.NoteBlocks`) _returnvalue_10)))))))))))

(event `/Game/char-select/Interface-char-select.game-lose`
  ; Spawn notes
  (for _array_element (`self.NoteBlocks`)
    (if (`KismetSystemLibrary.IsValid` _array_element)
      (bind _asactor (cast `Actor` _array_element))
      (`self.K2_DestroyActor` _asactor)))
  (`self.K2_DestroyActor`))

(fn `DestroyNoteBlocks`
  (for _array_element (`self.NoteBlocks`)
    (if (`KismetSystemLibrary.IsValid` _array_element)
      (bind _asactor (cast `Actor` _array_element))
      (`self.K2_DestroyActor` _asactor)))
  (return))

(fn `get-char`
  (returns (`char-output` :type "Array of /Game/char-select/char-select Object Reference"))
  (return))

(fn `UserConstructionScript`)